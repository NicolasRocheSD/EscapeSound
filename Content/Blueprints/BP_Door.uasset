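; Door actor that swings open a single time when its Interact event fires.
; BeginPlay stores the starting rotation, and a DoOnce on Interact lets it play interact and open sounds, then start the Opening timeline.
; The timeline lerps the whole actor's yaw a quarter turn from that stored rotation; there is no closing or reset logic.
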(event `self.ReceiveBeginPlay`
  (set `self.StartingRotation` (`self.K2_GetActorRotation`)))

(event `/Game/Blueprints/BPI_Interaction.Interact`
  (bind _returnvalue (`self.K2_GetActorLocation`))
  (bind (_startingrotation_roll _startingrotation_pitch _startingrotation_yaw) (`KismetMathLibrary.BreakRotator` (`self.StartingRotation`)))
  (`/Engine/EditorBlueprintResources/StandardMacros.DoOnce` false
    (:`Completed`
      (`GameplayStatics.PlaySoundAtLocation` "/Game/Audio/SFX/SFX_Door/SFX_Door_Interact.SFX_Door_Interact" _returnvalue (struct) 0.2 1.0 0.0 null null null null)
      (`GameplayStatics.PlaySoundAtLocation` "/Game/Audio/SFX/SFX_Door/SFX_Door_Open.SFX_Door_Open" _returnvalue (struct) 0.2 1.0 0.0 null null null null)
      (bind (_direction _newtrack_0) (`Timeline|Opening`)
        (:`Update`
          (`self.K2_SetActorRotation` (`KismetMathLibrary.RLerp` (`self.StartingRotation`) (`KismetMathLibrary.MakeRotator` _startingrotation_roll _startingrotation_pitch (+ _startingrotation_yaw -90.0)) _newtrack_0 true)))))))

(fn `UserConstructionScript`)